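; AI commander companion that wanders in the lobby and, in other levels, follows the player and fights Hulk, Parasite and Stalker enemies.
; PawnSensing sets focus and found flags, which AIFollow turns into per-type delayed rifle loops, prioritising Hulk and line-tracing along control rotation.
; The player's follow order interrupts combat, and a shot counter periodically clears targets.
; Tick reports location, HP and death to the player, then destroys the dead commander.
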(event OnSeePawn(PawnSensing)
  (params (Pawn :type Pawn%20Object%20Reference))
  (bind _returnvalue (Game|GetCurrentLevelName true))
  (if (not (Utilities|Enum|Equal(Enum) _returnvalue "LobbyBase"))
    (if (not (Variables|Default|GetIsDead))
      (bind _asbp_hulk_character (Utilities|Casting|CastToBP_HulkCharacter Pawn)
        (:then
          (if (not (Variables|/Game/Movable/Zombie/BP_HulkCharacter.BP_HulkCharacter_C|GetIsDead _asbp_hulk_character))
            (Variables|/Game/Movable/Zombie/BP_HulkCharacter.BP_HulkCharacter_C|SetAmIfounded? _asbp_hulk_character true)
            (Utilities|FlowControl|DoOnce false
              (:Completed
                (Variables|Default|SetHulk%20Ref _asbp_hulk_character)
                (AI|SetFocus (.AsAIController (Utilities|Casting|CastToAIController (Pawn|GetController))) (Variables|Default|GetHulk%20Ref))
                (Variables|Default|SetIsFindHulk true)))))
        (:CastFailed
          (bind _asbp_parasite_character (Utilities|Casting|CastToBP_ParasiteCharacter Pawn)
            (:then
              (if (not (Variables|/Game/Movable/Zombie/BP_ParasiteCharacter.BP_ParasiteCharacter_C|GetIsDead _asbp_parasite_character))
                (Variables|/Game/Movable/Zombie/BP_ParasiteCharacter.BP_ParasiteCharacter_C|SetAmIFounded? _asbp_parasite_character true)
                (Utilities|FlowControl|DoOnce false
                  (:Completed
                    (Variables|Default|SetParasite%20Ref _asbp_parasite_character)
                    (AI|SetFocus (.AsAIController (Utilities|Casting|CastToAIController (Pawn|GetController))) (Variables|Default|GetParasite%20Ref))
                    (Variables|Default|SetIsFindParasite true)))))
            (:CastFailed
              (bind _asbp_stalker_character (Utilities|Casting|CastToBP_StalkerCharacter Pawn)
                (:then
                  (if (not (Variables|/Game/Movable/Zombie/BP_StalkerCharacter.BP_StalkerCharacter_C|GetIsDead _asbp_stalker_character))
                    (Variables|/Game/Movable/Zombie/BP_StalkerCharacter.BP_StalkerCharacter_C|SetAmIFounded? _asbp_stalker_character true)
                    (Utilities|FlowControl|DoOnce false
                      (:Completed
                        (Variables|Default|SetStalker%20Ref _asbp_stalker_character)
                        (AI|SetFocus (.AsAIController (Utilities|Casting|CastToAIController (Pawn|GetController))) (Variables|Default|GetStalker%20Ref))
                        (Variables|Default|SetIsFindStalker true)))))
                (:CastFailed
                  (Utilities|FlowControl|Delay 4.0)
                  (CallFunction|AIFollow))))))))))

(event Custom|AIFollow
  (|OderFollow?_3_2_2)
  (if (not (Variables|Default|GetIsDead))
    (Utilities|FlowControl|Sequence
      (:then_0
        (if (Variables|Default|GetIsFindHulk)
          (Variables|Default|SetNowAIfollow? false)
          (CallFunction|HulkShotStart)
          (elif (Variables|Default|GetIsFindParasite)
            (Variables|Default|SetNowAIfollow? false)
            (CallFunction|ParasiteShotStart)
            (elif (Variables|Default|GetIsFindStalker)
              (Variables|Default|SetNowAIfollow? false)
              (CallFunction|StalkerShotStart)
              (else
                (Variables|Default|SetNowAIfollow? true)
                (AI|AIMoveTo self (CallFunction|GetRandomPosAroundPlayer) 0 5.0 false
                  (:then
                    (Variables|Default|SetStillAIFollow%20On? true))
                  (:OnSuccess
                    (if (CallFunction|IsPlayerClose) :!label _label
                      (Utilities|FlowControl|Delay 4.0)
                      (CallFunction|AIFollow)
                      (else
                        (CallFunction|AIFollow))))
                  (:OnFail
                    (goto _label)))))))))))

(event Custom|ResetStalkerShot
  (Utilities|FlowControl|DoOnce false) ; enters at Reset
)

(event Custom|ParasiteShotStart
  (|OderFollow2_2_2
    (:else
      (if (not (Variables|Default|GetIsDead))
        (|ParasiteShot)))))

(event Custom|ResetHulkShot
  (Utilities|FlowControl|DoOnce false) ; enters at Reset
)

(event Custom|ResetParasiteShot
  (Utilities|FlowControl|DoOnce false) ; enters at Reset
)

(event Custom|ResetHulkSensing
  (Utilities|FlowControl|DoOnce false) ; enters at Reset
)

(event Custom|ResetStalkerSensing
  (Utilities|FlowControl|DoOnce false) ; enters at Reset
)

(event Custom|StalkerShotStart
  (|OderFollow3_2_2
    (:else
      (if (not (Variables|Default|GetIsDead))
        (|StalkerShot)))))

(event Custom|ResetParasiteSensing
  (Utilities|FlowControl|DoOnce false) ; enters at Reset
)

(event Custom|HulkShotStart
  (|OderFollow_2_2
    (:else
      (if (not (Variables|Default|GetIsDead))
        (|HulkShot)))))

(event EventBeginPlay
  (Variables|Default|SetCurrent%20HP (Variables|Default|GetMax%20HP))
  (bind _returnvalue (Game|GetCurrentLevelName true))
  (if (Utilities|Enum|Equal(Enum) _returnvalue "LobbyBase")
    (AI|AIMoveTo self (.RandomLocation (AI|Navigation|GetRandomReachablePointinRadius (Transformation|GetActorLocation) 1e+03 0 "/Script/AIModule.NavFilter_AIControllerDefault")) 0 5.0 false :!label _label
      (:OnSuccess
        _)
      (:OnFail
        _))
    (Utilities|FlowControl|Delay 3.0)
    (AI|AIMoveTo self (.RandomLocation (AI|Navigation|GetRandomReachablePointinRadius (Transformation|GetActorLocation) 1e+03 0 "/Script/AIModule.NavFilter_AIControllerDefault")) 0 5.0 false
      (:OnSuccess
        (goto _label))
      (:OnFail
        (goto _label)))
    (else
      (CallFunction|AIFollow))))

(event EventTick
  (params (DeltaSeconds :type Float%20%28single-precision%29))
  (bind _returnvalue (Transformation|GetActorRotation))
  (bind (_roll _pitch) (Math|Rotator|BreakRotator _returnvalue))
  (bind _returnvalue_2 (Game|GetCurrentLevelName true))
  (if (not (Utilities|Enum|Equal(Enum) _returnvalue_2 "LobbyBase"))
    (bind _asbp_player_charactor (Utilities|Casting|CastToBP_PlayerCharactor (Game|GetPlayerCharacter 0)))
    (Variables|/Game/Movable/Charactor/BP_PlayerCharactor.BP_PlayerCharactor_C|SetForEnemySendCommanderLocation _asbp_player_charactor (Transformation|GetActorLocation))
    (if (not (Variables|Default|GetIsDead))
      (|SendHPToPlayer)
      (if (> (Variables|Default|GetCurrent%20HP) 0.0)
        (Utilities|Casting|CastToBP_PlayerCharactor (Game|GetPlayerCharacter 0))
        (if (< (Math|Vector|VectorLength (Transformation|GetVelocity)) 5e+01)
          (Utilities|FlowControl|Sequence
            (:then_0
              (if (Variables|Default|GetNowAIfollow?)
                (Transformation|SetActorRotation (Math|Rotator|MakeRotator _roll _pitch (.Yaw (Math|Rotator|BreakRotator (Math|Interpolation|RInterpTo _returnvalue (Math|Rotator|FindLookatRotation (Transformation|GetActorLocation) (Transformation|GetActorLocation (Game|GetPlayerCharacter 0))) DeltaSeconds 1e+01)))))
                (else
                  (Utilities|FlowControl|Sequence
                    (:then_0
                      (if (not (Variables|Default|GetIsFindHulk))
                        (Utilities|FlowControl|DoOnce false
                          (:Completed
                            (Utilities|FlowControl|Sequence
                              (:then_0
                                (if (== (Math|Random|RandomIntegerinRange 0 4) 0)
                                  _)))))))
                    (:then_1
                      (if (not (Variables|Default|GetIsFindParasite))
                        (Utilities|FlowControl|DoOnce false
                          (:Completed
                            (Utilities|FlowControl|Sequence
                              (:then_0
                                (if (== (Math|Random|RandomIntegerinRange 0 4) 0)
                                  _)))))))
                    (:then_2
                      (if (not (Variables|Default|GetIsFindStalker))
                        (Utilities|FlowControl|DoOnce false
                          (:Completed
                            (Utilities|FlowControl|Sequence
                              (:then_0
                                (if (== (Math|Random|RandomIntegerinRange 0 4) 0)
                                  _)))))))
                    (:then_3
                      (if (Math|Boolean|ANDBoolean (Variables|Default|GetIsFindParasite) (Variables|Default|GetIsFindHulk) (Variables|Default|GetIsFindStalker))
                        (if (not (Variables|Default|GetStillAIFollow%20On?))
                          (CallFunction|AIFollow))))))))
            (:then_1
              (|5발이상아무것도못맞추면타겟재설정))))
        (else
          (Variables|Default|SetIsDead true)
          (Components|Movement|StopMovementImmediately (Variables|Character|GetCharacterMovement))
          (bind _asbp_player_charactor_2 (Utilities|Casting|CastToBP_PlayerCharactor (Game|GetPlayerCharacter 0)))
          (Variables|/Game/Movable/Charactor/BP_PlayerCharactor.BP_PlayerCharactor_C|SetForEnemySendCommanderIsDead _asbp_player_charactor_2 true)
          (Animation|PlayAnimMontage "/Game/Movable/CharactorAsset/Commander/Commander_Animation/Die_Montage.Die_Montage" 1.0 "None")
          (Utilities|FlowControl|Delay 1.5)
          (Actor|DestroyActor))))))

(fn ConstructionScript)

(fn GetRandomPosAroundPlayer
  (return (.RandomLocation (Class|NavigationSystemV1|GetRandomPointinNavigableRadius (Transformation|GetActorLocation (Game|GetPlayerCharacter 0)) 6e+02 0 0))))

(fn IsPlayerClose
  (return (<= (Transformation|GetDistanceTo (Game|Player|GetPlayerPawn 0) self) 6.5e+02)))