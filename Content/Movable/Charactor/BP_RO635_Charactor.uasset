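; RO635 AI companion character that follows the player and shoots Hulk, Parasite and Stalker enemies.
; It moves to random navmesh points near the player until PawnSensing spots an enemy and sets AI focus.
; Per-enemy-type recursive fire loops apply line-trace damage until the target is invalid; a Hulk-shot counter also forces retargeting.
; Tick reports location, HP and death to the player, turns toward them, plays voice lines and handles dying.
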(event OnSeePawn(PawnSensing)
  (params (Pawn :type Pawn%20Object%20Reference))
  (if (not (Variables|Default|GetIsDead))
    (bind _asbp_hulk_character (Utilities|Casting|CastToBP_HulkCharacter Pawn)
      (:then
        (if (not (Variables|/Game/Movable/Zombie/BP_HulkCharacter.BP_HulkCharacter_C|GetIsDead _asbp_hulk_character))
          (Variables|/Game/Movable/Zombie/BP_HulkCharacter.BP_HulkCharacter_C|SetAmIfounded? _asbp_hulk_character true)
          (Utilities|FlowControl|DoOnce false
            (:Completed
              (Variables|Default|SetHulk%20Ref _asbp_hulk_character)
              (AI|SetFocus (.AsAIController (Utilities|Casting|CastToAIController (Pawn|GetController))) (Variables|Default|GetHulk%20Ref))
              (Variables|Default|SetIsFindHulk true)))))
      (:CastFailed
        (bind _asbp_parasite_character (Utilities|Casting|CastToBP_ParasiteCharacter Pawn)
          (:then
            (if (not (Variables|/Game/Movable/Zombie/BP_ParasiteCharacter.BP_ParasiteCharacter_C|GetIsDead _asbp_parasite_character))
              (Variables|/Game/Movable/Zombie/BP_ParasiteCharacter.BP_ParasiteCharacter_C|SetAmIFounded? _asbp_parasite_character false)
              (Utilities|FlowControl|DoOnce false
                (:Completed
                  (Variables|Default|SetParasite%20Ref _asbp_parasite_character)
                  (AI|SetFocus (.AsAIController (Utilities|Casting|CastToAIController (Pawn|GetController))) (Variables|Default|GetParasite%20Ref))
                  (Variables|Default|SetIsFindParasite true)))))
          (:CastFailed
            (bind _asbp_stalker_character (Utilities|Casting|CastToBP_StalkerCharacter Pawn)
              (:then
                (if (not (Variables|/Game/Movable/Zombie/BP_StalkerCharacter.BP_StalkerCharacter_C|GetIsDead _asbp_stalker_character))
                  (Variables|/Game/Movable/Zombie/BP_StalkerCharacter.BP_StalkerCharacter_C|SetAmIFounded? _asbp_stalker_character false)
                  (Utilities|FlowControl|DoOnce false
                    (:Completed
                      (Variables|Default|SetStalker%20Ref _asbp_stalker_character)
                      (AI|SetFocus (.AsAIController (Utilities|Casting|CastToAIController (Pawn|GetController))) (Variables|Default|GetStalker%20Ref))
                      (Variables|Default|SetIsFindStalker true)))))
              (:CastFailed
                (CallFunction|AIFollow)))))))))

(event Custom|AIFollow
  (if (not (Variables|Default|GetIsDead))
    (Utilities|FlowControl|Sequence
      (:then_0
        (if (Variables|Default|GetIsFindHulk)
          (Variables|Default|SetNowAIfollow? false)
          (CallFunction|HulkShotStart)
          (else
            (Variables|Default|SetNowAIfollow? true)
            (AI|AIMoveTo self (CallFunction|GetRandomPosAroundPlayer) 0 5.0 false
              (:OnSuccess
                _)
              (:OnFail
                _))
            (Variables|Default|SetStillAIFollow%20On? true))))
      (:then_1
        (if (Variables|Default|GetIsFindParasite)
          (Variables|Default|SetNowAIfollow? false)
          (CallFunction|ParasiteShotStart)
          (else
            (Variables|Default|SetNowAIfollow? true)
            (AI|AIMoveTo self (CallFunction|GetRandomPosAroundPlayer) 0 5.0 false
              (:OnSuccess
                _)
              (:OnFail
                _))
            (Variables|Default|SetStillAIFollow%20On? true))))
      (:then_2
        (if (Variables|Default|GetIsFindStalker)
          (Variables|Default|SetNowAIfollow? false)
          (CallFunction|StalkerShotStart)
          (else
            (Variables|Default|SetNowAIfollow? true)
            (AI|AIMoveTo self (CallFunction|GetRandomPosAroundPlayer) 0 5.0 false
              (:OnSuccess
                _)
              (:OnFail
                _))
            (Variables|Default|SetStillAIFollow%20On? true)
            (if (CallFunction|IsPlayerClose)
              (Utilities|FlowControl|Delay 1.0)
              (CallFunction|AIFollow)
              (else
                (CallFunction|AIFollow)))))))))

(event Custom|ResetStalkerShot
  (Utilities|FlowControl|DoOnce false) ; enters at Reset
)

(event Custom|ParasiteShotStart
  (if (not (Variables|Default|GetIsDead))
    (|ParasiteShot)))

(event Custom|ResetHulkShot
  (Utilities|FlowControl|DoOnce false) ; enters at Reset
)

(event Custom|ResetParasiteShot
  (Utilities|FlowControl|DoOnce false) ; enters at Reset
)

(event Custom|ResetHulkSensing
  (Utilities|FlowControl|DoOnce false) ; enters at Reset
)

(event Custom|ResetStalkerSensing
  (Utilities|FlowControl|DoOnce false) ; enters at Reset
)

(event Custom|StalkerShotStart
  (if (not (Variables|Default|GetIsDead))
    (|StalkerShot)))

(event Custom|ResetParasiteSensing
  (Utilities|FlowControl|DoOnce false) ; enters at Reset
)

(event Custom|HulkShotStart
  (if (not (Variables|Default|GetIsDead))
    (|HulkShot)))

(event EventBeginPlay
  (Variables|Default|SetCurrent%20HP (Variables|Default|GetMax%20HP))
  (CallFunction|AIFollow))

(event EventTick
  (params (DeltaSeconds :type Float%20%28single-precision%29))
  (bind _returnvalue (Transformation|GetActorRotation))
  (bind (_roll _pitch) (Math|Rotator|BreakRotator _returnvalue))
  (bind _asbp_player_charactor (Utilities|Casting|CastToBP_PlayerCharactor (Game|GetPlayerCharacter 0)))
  (Variables|/Game/Movable/Charactor/BP_PlayerCharactor.BP_PlayerCharactor_C|SetForEnemySendRO635Loctaion _asbp_player_charactor (Transformation|GetActorLocation))
  (if (not (Variables|Default|GetIsDead))
    (|SendHPToPlayer)
    (if (> (Variables|Default|GetCurrent%20HP) 0.0)
      (Utilities|Casting|CastToBP_PlayerCharactor (Game|GetPlayerCharacter 0))
      (if (< (Math|Vector|VectorLength (Transformation|GetVelocity)) 5e+01)
        (Utilities|FlowControl|Sequence
          (:then_0
            (if (Variables|Default|GetNowAIfollow?)
              (Transformation|SetActorRotation (Math|Rotator|MakeRotator _roll _pitch (.Yaw (Math|Rotator|BreakRotator (Math|Interpolation|RInterpTo _returnvalue (Math|Rotator|FindLookatRotation (Transformation|GetActorLocation) (Transformation|GetActorLocation (Game|GetPlayerCharacter 0))) DeltaSeconds 1e+01)))))
              (else
                (Utilities|FlowControl|Sequence
                  (:then_0
                    (if (not (Variables|Default|GetIsFindHulk))
                      (Utilities|FlowControl|DoOnce false
                        (:Completed
                          (Utilities|FlowControl|Sequence
                            (:then_0
                              (if (== (Math|Random|RandomIntegerinRange 0 4) 0)
                                (Audio|PlaySoundatLocation "/Game/Movable/CharactorAsset/RO635/RO635_Sound/RO635_SKILL1_JP.RO635_SKILL1_JP" (Transformation|GetActorLocation) "0, 0, 0" 1.0 1.0 0.0 0 0 0))))))))
                  (:then_1
                    (if (not (Variables|Default|GetIsFindParasite))
                      (Utilities|FlowControl|DoOnce false
                        (:Completed
                          (Utilities|FlowControl|Sequence
                            (:then_0
                              (if (== (Math|Random|RandomIntegerinRange 0 4) 0)
                                (Audio|PlaySoundatLocation "/Game/Movable/CharactorAsset/G36C/G36C_Sound/G36C_ShotVoice_Cue.G36C_ShotVoice_Cue" (Transformation|GetActorLocation) "0, 0, 0" 1.0 1.0 0.0 0 0 0))))))))
                  (:then_2
                    (if (not (Variables|Default|GetIsFindStalker))
                      (Utilities|FlowControl|DoOnce false
                        (:Completed
                          (Utilities|FlowControl|Sequence
                            (:then_0
                              (if (== (Math|Random|RandomIntegerinRange 0 4) 0)
                                (Audio|PlaySoundatLocation "/Game/Movable/CharactorAsset/G36C/G36C_Sound/G36C_ShotVoice_Cue.G36C_ShotVoice_Cue" (Transformation|GetActorLocation) "0, 0, 0" 1.0 1.0 0.0 0 0 0))))))))
                  (:then_3
                    (if (Math|Boolean|ANDBoolean (Variables|Default|GetIsFindParasite) (Variables|Default|GetIsFindHulk) (Variables|Default|GetIsFindStalker))
                      (if (not (Variables|Default|GetStillAIFollow%20On?))
                        (CallFunction|AIFollow))))))))
          (:then_1
            (|5발이상못맞출경우타겟재설정))))
      (else
        (Variables|Default|SetIsDead true)
        (Components|Movement|StopMovementImmediately (Variables|Character|GetCharacterMovement))
        (bind _asbp_player_charactor_2 (Utilities|Casting|CastToBP_PlayerCharactor (Game|GetPlayerCharacter 0)))
        (Variables|/Game/Movable/Charactor/BP_PlayerCharactor.BP_PlayerCharactor_C|SetForEnemySendRO635IsDead _asbp_player_charactor_2 true)
        (Animation|PlayAnimMontage "/Game/Movable/CharactorAsset/RO635/RO635_Animation/Dying_Montage.Dying_Montage" 1.0 "None")
        (Utilities|FlowControl|Delay 3.5)
        (Actor|DestroyActor)))))

(fn ConstructionScript)

(fn GetRandomPosAroundPlayer
  (return (.RandomLocation (Class|NavigationSystemV1|GetRandomPointinNavigableRadius (Transformation|GetActorLocation (Game|GetPlayerCharacter 0)) 6e+02 0 0))))

(fn IsPlayerClose
  (return (<= (Transformation|GetDistanceTo (Game|Player|GetPlayerPawn 0) self) 6.5e+02)))