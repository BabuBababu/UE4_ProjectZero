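; Parasite zombie enemy character that wanders to random reachable points until damaged, then chases and melees the player.
; AIMoveTo loops drive roaming and hunting, with random left or right attack montages on reaching the player.
; Hand overlaps subtract player HP while the Attack flag, toggled by OnAttack/OffAttack events, is set.
; Point damage updates a health bar widget; at zero health it stops, disables collision and is destroyed after a random delay.
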(event OnComponentBeginOverlap(LHand)
  (params (OverlappedComponent :type Primitive%20Component%20Object%20Reference) (OtherActor :type Actor%20Object%20Reference) (OtherComp :type Primitive%20Component%20Object%20Reference) (OtherBodyIndex :type Integer) (bFromSweep :type Boolean) (SweepResult :type Hit%20Result%20Structure%20%28by%20ref%29))
  (if (Variables|Default|GetAttack)
    (bind _asbp_player_charactor (Utilities|Casting|CastToBP_PlayerCharactor OtherActor))
    (Variables|/Game/Movable/Charactor/BP_PlayerCharactor.BP_PlayerCharactor_C|SetCurrentHP _asbp_player_charactor (- (Variables|/Game/Movable/Charactor/BP_PlayerCharactor.BP_PlayerCharactor_C|GetCurrentHP _asbp_player_charactor) 1e+01))
    (Variables|/Game/Movable/Charactor/BP_PlayerCharactor.BP_PlayerCharactor_C|SetIsHurted _asbp_player_charactor true)))

(event OnComponentBeginOverlap(RHand)
  (params (OverlappedComponent :type Primitive%20Component%20Object%20Reference) (OtherActor :type Actor%20Object%20Reference) (OtherComp :type Primitive%20Component%20Object%20Reference) (OtherBodyIndex :type Integer) (bFromSweep :type Boolean) (SweepResult :type Hit%20Result%20Structure%20%28by%20ref%29))
  (if (Variables|Default|GetAttack)
    (bind _asbp_player_charactor (Utilities|Casting|CastToBP_PlayerCharactor OtherActor))
    (Variables|/Game/Movable/Charactor/BP_PlayerCharactor.BP_PlayerCharactor_C|SetCurrentHP _asbp_player_charactor (- (Variables|/Game/Movable/Charactor/BP_PlayerCharactor.BP_PlayerCharactor_C|GetCurrentHP _asbp_player_charactor) 1e+01))
    (Variables|/Game/Movable/Charactor/BP_PlayerCharactor.BP_PlayerCharactor_C|SetIsHurted _asbp_player_charactor true)))

(event Custom|OffAttack
  (Variables|Default|SetAttack false))

(event Custom|AIMovement
  (if (not (Variables|Default|GetIsDead))
    (Audio|PlaySoundatLocation "/Game/Movable/ZombieAsset/ZombieSound/Parasite_Walking_Sound_Cue.Parasite_Walking_Sound_Cue" (Transformation|GetActorLocation) "0, 0, 0" 1.0 1.0 0.0 0 0 0)
    (if (not (Variables|Default|GetEnemyFound))
      (AI|AIMoveTo self (.RandomLocation (AI|Navigation|GetRandomReachablePointinRadius (Transformation|GetActorLocation) 3e+04 0 "/Script/AIModule.NavFilter_AIControllerDefault")) 0 5.0 false
        (:OnSuccess
          (Utilities|FlowControl|Delay (Math|Random|RandomFloatinRange 2.0 6.0) :!label _label)
          (CallFunction|AIMovement))
        (:OnFail
          (if (not (Variables|Default|GetIsDead))
            (if (not (Variables|Default|GetEnemyFound))
              (goto _label))))))))

(event Custom|AttackPlayer
  (Audio|PlaySoundatLocation "/Game/Movable/ZombieAsset/ZombieSound/Prasite_Attack_Sound_Cue.Prasite_Attack_Sound_Cue" (Transformation|GetActorLocation) "0, 0, 0" 1.0 1.0 0.0 0 0 0)
  (switch int (Math|Random|RandomIntegerinRange 0 1)
    (:0
      (bind _returnvalue (Animation|PlayAnimMontage "/Game/Movable/ZombieAsset/ZombieAnimation/Zombie_Attack_L_Montage.Zombie_Attack_L_Montage" 1.0 "None"))
      (Utilities|FlowControl|Delay _returnvalue))
    (:1
      (bind _returnvalue_2 (Animation|PlayAnimMontage "/Game/Movable/ZombieAsset/ZombieAnimation/Zombie_Attack_R_Montage.Zombie_Attack_R_Montage" 1.0 "None"))
      (Utilities|FlowControl|Delay _returnvalue_2)))
  (CallFunction|HuntPlayer))

(event Custom|HuntPlayer
  (if (not (Variables|Default|GetIsDead))
    (Variables|/Script/Engine.CharacterMovementComponent|SetMaxWalkSpeed (Variables|Character|GetCharacterMovement) 4e+02)
    (AI|AIMoveTo self "0, 0, 0" (Game|GetPlayerCharacter 0) 5e+01 true
      (:OnSuccess
        (CallFunction|AttackPlayer))
      (:OnFail
        (CallFunction|HuntPlayer)))))

(event Custom|OnAttack
  (Variables|Default|SetAttack true))

(event EventBeginPlay
  (Variables|Default|SetCurrentHealth (Variables|Default|GetMaxHealth))
  (CallFunction|AIMovement)
  (CallFunction|UpdateHealth))

(event Game|Damage|EventPointDamage
  (params (Damage :type Float%20%28single-precision%29) (DamageType :type Damage%20Type%20Object%20Reference) (HitLocation :type Vector :default "0, 0, 0") (HitNormal :type Vector :default "0, 0, 0") (HitComponent :type Primitive%20Component%20Object%20Reference) (BoneName :type Name :default "None") (ShotFromDirection :type Vector :default "0, 0, 0") (InstigatedBy :type Controller%20Object%20Reference) (DamageCauser :type Actor%20Object%20Reference) (HitInfo :type Hit%20Result%20Structure%20%28by%20ref%29))
  (Variables|Default|SetCurrentHealth (- (Variables|Default|GetCurrentHealth) Damage))
  (CallFunction|UpdateHealth)
  (Utilities|FlowControl|Sequence
    (:then_0
      (if (<= (Variables|Default|GetCurrentHealth) 0.0)
        (Variables|Default|SetIsDead true)
        (Components|Movement|StopMovementImmediately (Variables|Character|GetCharacterMovement))
        (Collision|SetCollisionEnabled (Variables|Collision|GetCapsuleComponent) "NoCollision")
        (Utilities|FlowControl|Delay (Math|Random|RandomFloatinRange 2.0 5.0))
        (Actor|DestroyActor)))
    (:then_1
      (bind _output_get (Variables|Default|SetEnemyFound true))
      (if _output_get
        (Utilities|FlowControl|DoOnce false
          (:Completed
            (CallFunction|HuntPlayer)))))))

(fn ConstructionScript)

(fn UpdateHealth
  (bind _asbp_parasite_widget (Utilities|Casting|CastToBP_Parasite_Widget (UserInterface|GetUserWidgetObject (Variables|Default|GetWidget))))
  (Progress|SetPercent (Variables|/Game/Movable/Zombie/BP_Parasite_Widget.BP_Parasite_Widget_C|GetHealthBar _asbp_parasite_widget) (/ (Variables|Default|GetCurrentHealth) (Variables|Default|GetMaxHealth)))
  (if (<= (Variables|Default|GetCurrentHealth) 0.0)
    (Rendering|SetVisibility (Variables|Default|GetWidget) false false)))