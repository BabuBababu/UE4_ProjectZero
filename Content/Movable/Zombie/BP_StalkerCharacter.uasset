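; Stalker zombie enemy that wanders the navmesh and chases the player once it sees them or takes damage.
; Recursive AI MoveTo events drive wandering and hunting, while Tick uses DoOnce gates to switch between them, returning to wandering when the player is distant or dead.
; Overlapping its UpperBody damages the player and destroys the stalker in an impact effect.
; Point damage updates a proximity-shown health bar widget and handles delayed death.
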(event OnComponentEndOverlap(UpperBody)
  (params (OverlappedComponent :type Primitive%20Component%20Object%20Reference) (OtherActor :type Actor%20Object%20Reference) (OtherComp :type Primitive%20Component%20Object%20Reference) (OtherBodyIndex :type Integer))
  (Utilities|Casting|CastToBP_PlayerCharactor OtherActor)
  (Variables|Default|SetOverlap false))

(event OnSeePawn(PawnSensing)
  (params (Pawn :type Pawn%20Object%20Reference))
  (if (not (Variables|Default|GetIsDead))
    (bind _asbp_player_charactor (Utilities|Casting|CastToBP_PlayerCharactor Pawn))
    (if (not (Variables|/Game/Movable/Charactor/BP_PlayerCharactor.BP_PlayerCharactor_C|GetIsDead _asbp_player_charactor))
      (Utilities|FlowControl|DoOnce false
        (:Completed
          (Variables|Default|SetEnemyFound true))))))

(event OnComponentBeginOverlap(UpperBody)
  (params (OverlappedComponent :type Primitive%20Component%20Object%20Reference) (OtherActor :type Actor%20Object%20Reference) (OtherComp :type Primitive%20Component%20Object%20Reference) (OtherBodyIndex :type Integer) (bFromSweep :type Boolean) (SweepResult :type Hit%20Result%20Structure%20%28by%20ref%29))
  (Utilities|Casting|CastToBP_PlayerCharactor OtherActor)
  (Variables|Default|SetOverlap true))

(event Custom|AIMovement
  (if (not (Variables|Default|GetIsDead))
    (if (not (Variables|Default|GetEnemyFound))
      (AI|AIMoveTo self (.RandomLocation (AI|Navigation|GetRandomReachablePointinRadius (Transformation|GetActorLocation) 3e+04 0 "/Script/AIModule.NavFilter_AIControllerDefault")) 0 5.0 false
        (:OnSuccess
          (Utilities|FlowControl|Delay (Math|Random|RandomFloatinRange 2.0 6.0) :!label _label)
          (CallFunction|AIMovement))
        (:OnFail
          (if (not (Variables|Default|GetIsDead))
            (if (not (Variables|Default|GetEnemyFound))
              (goto _label))))))))

(event Custom|AttackPlayer
  (Audio|PlaySoundatLocation "/Game/Movable/ZombieAsset/Stalker/Sound/Stalker_Attack_Cue.Stalker_Attack_Cue" (Transformation|GetActorLocation) "0, 0, 0" 1.0 1.0 0.0 0 0 0)
  (Animation|PlayAnimMontage "/Game/Movable/ZombieAsset/Stalker/Animation/Stalker_Attack_Montage.Stalker_Attack_Montage" 1.0 "None")
  (Utilities|FlowControl|Delay 0.5)
  (CallFunction|HuntPlayer))

(event Custom|HuntPlayer
  (if (not (Variables|Default|GetIsDead))
    (if (Variables|Default|GetEnemyFound)
      (Audio|PlaySoundatLocation "/Game/Movable/ZombieAsset/Stalker/Sound/Stalker_Run_Cue.Stalker_Run_Cue" (Transformation|GetActorLocation) "0, 0, 0" 1.0 1.0 0.0 0 0 0)
      (Variables|/Script/Engine.CharacterMovementComponent|SetMaxWalkSpeed (Variables|Character|GetCharacterMovement) 6e+02)
      (AI|AIMoveTo self "0, 0, 0" (Game|GetPlayerCharacter 0) 5e+01 true
        (:OnSuccess
          (CallFunction|AttackPlayer))
        (:OnFail
          (if (Variables|Default|GetEnemyFound)
            (Utilities|FlowControl|Delay 0.2)
            (CallFunction|HuntPlayer)))))))

(event Custom|ResetPawnSensing
  (Utilities|FlowControl|DoOnce false) ; enters at Reset
)

(event EventBeginPlay
  (bind _output_get (Variables|Default|SetCurrentHealth (Variables|Default|GetMaxHealth)))
  (Development|PrintString (Utilities|String|ToString(Float) _output_get))
  (CallFunction|AIMovement)
  (CallFunction|UpdateHealth))

(event EventTick
  (params (DeltaSeconds :type Float%20%28single-precision%29))
  (bind _returnvalue (Transformation|GetActorLocation))
  (if (Variables|/Game/Movable/Charactor/BP_PlayerCharactor.BP_PlayerCharactor_C|GetIsDead (.AsBP%20Player%20Charactor (Utilities|Casting|CastToBP_PlayerCharactor (Game|GetPlayerCharacter 0))))
    (Utilities|FlowControl|DoOnce false
      (:Completed
        (CallFunction|ResetPawnSensing)
        (Variables|Default|SetEnemyFound false)
        (Variables|/Script/Engine.CharacterMovementComponent|SetMaxWalkSpeed (Variables|Character|GetCharacterMovement) 1e+02)
        (Components|Movement|StopMovementImmediately (Variables|Character|GetCharacterMovement))
        (Utilities|FlowControl|Delay (Math|Random|RandomFloatinRange 2.0 4.0))
        (AI|SetFocus (.AsAIController (Utilities|Casting|CastToAIController (Pawn|GetController))))
        (CallFunction|AIMovement)))
    (elif (not (Variables|Default|GetIsDead))
      (Utilities|FlowControl|Sequence
        (:then_0
          (if (Variables|Default|GetEnemyFound)
            (Utilities|FlowControl|DoOnce false :!label _label
              (:Completed
                (AI|SetFocus (.AsAIController (Utilities|Casting|CastToAIController (Pawn|GetController))) (Game|GetPlayerCharacter 0))
                (CallFunction|HuntPlayer)))
            (else
              (goto _label Reset))))
        (:then_1
          (if (>= (Transformation|GetDistanceTo (.AsBP%20Player%20Charactor (Utilities|Casting|CastToBP_PlayerCharactor (Game|GetPlayerCharacter 0)))) 1e+03)
            (Utilities|FlowControl|Sequence
              (:then_0
                (Utilities|FlowControl|DoOnce false :!label _label_2
                  (:Completed
                    (Variables|Default|SetEnemyFound false)
                    (CallFunction|ResetPawnSensing)
                    (Components|Movement|StopMovementImmediately (Variables|Character|GetCharacterMovement))
                    (Variables|/Script/Engine.CharacterMovementComponent|SetMaxWalkSpeed (Variables|Character|GetCharacterMovement) 1e+02)
                    (AI|SetFocus (.AsAIController (Utilities|Casting|CastToAIController (Pawn|GetController))))
                    (Utilities|FlowControl|Delay (Math|Random|RandomFloatinRange 2.0 6.0))
                    (CallFunction|AIMovement))))
              (:then_1
                (Utilities|FlowControl|DoOnce false :!label _label_3
                  (:Completed
                    (Rendering|SetVisibility (Variables|Default|GetWidget) false false)))))
            (else
              (Utilities|FlowControl|Sequence
                (:then_0
                  (goto _label_2 Reset))
                (:then_1
                  (Rendering|SetVisibility (Variables|Default|GetWidget) true false)
                  (goto _label_3 Reset))))))
        (:then_2
          (if (Variables|Default|GetOverlap)
            (Audio|PlaySoundatLocation "/Game/Movable/ZombieAsset/Stalker/Sound/Stalker_Attack_Cue.Stalker_Attack_Cue" _returnvalue "0, 0, 0" 1.0 1.0 0.0 0 0 0)
            (Effects|SpawnEmitteratLocation "/Game/Movable/WeaponAsset/WeaponEffects/P_body_bullet_impact_2.P_body_bullet_impact_2" _returnvalue "0, 0, 0" "5.000000,5.000000,5.000000")
            (bind _asbp_player_charactor (Utilities|Casting|CastToBP_PlayerCharactor (Game|GetPlayerCharacter 0)))
            (Variables|/Game/Movable/Charactor/BP_PlayerCharactor.BP_PlayerCharactor_C|SetCurrentHP _asbp_player_charactor (- (Variables|/Game/Movable/Charactor/BP_PlayerCharactor.BP_PlayerCharactor_C|GetCurrentHP _asbp_player_charactor) 4e+01))
            (Variables|/Game/Movable/Charactor/BP_PlayerCharactor.BP_PlayerCharactor_C|SetIsHurted _asbp_player_charactor true)
            (Actor|DestroyActor)))))))

(event Game|Damage|EventPointDamage
  (params (Damage :type Float%20%28single-precision%29) (DamageType :type Damage%20Type%20Object%20Reference) (HitLocation :type Vector :default "0, 0, 0") (HitNormal :type Vector :default "0, 0, 0") (HitComponent :type Primitive%20Component%20Object%20Reference) (BoneName :type Name :default "None") (ShotFromDirection :type Vector :default "0, 0, 0") (InstigatedBy :type Controller%20Object%20Reference) (DamageCauser :type Actor%20Object%20Reference) (HitInfo :type Hit%20Result%20Structure%20%28by%20ref%29))
  (Variables|Default|SetCurrentHealth (- (Variables|Default|GetCurrentHealth) Damage))
  (CallFunction|UpdateHealth)
  (Variables|Default|SetEnemyFound true)
  (if (<= (Variables|Default|GetCurrentHealth) 0.0)
    (Variables|Default|SetIsDead true)
    (Components|Movement|StopMovementImmediately (Variables|Character|GetCharacterMovement))
    (Collision|SetCollisionEnabled (Variables|Collision|GetCapsuleComponent) "NoCollision")
    (Utilities|FlowControl|Delay (Math|Random|RandomFloatinRange 1.5 3.0))
    (Actor|DestroyActor)))

(fn ConstructionScript)

(fn UpdateHealth
  (bind _asbp_zombie_widget (Utilities|Casting|CastToBP_Zombie_Widget (UserInterface|GetUserWidgetObject (Variables|Default|GetWidget))))
  (Progress|SetPercent (Variables|/Game/Movable/Zombie/BP_Zombie_Widget.BP_Zombie_Widget_C|GetHealthBar _asbp_zombie_widget) (/ (Variables|Default|GetCurrentHealth) (Variables|Default|GetMaxHealth)))
  (if (<= (Variables|Default|GetCurrentHealth) 0.0)
    (Rendering|SetVisibility (Variables|Default|GetWidget) false false)))